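; NPC character Blueprint that shows a selection indicator and a quest-state marker.
; On BeginPlay it caches the game instance, cast to RootsOfShadowsGameState.
; OnQuestUIChanged hides all four quest widgets (GE, GI, YE, YI), then shows the one matching QuestState.
; Tick syncs selection visibility to IsSelected and rotates any visible quest widget toward the player camera manager.
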(event EventBeginPlay
  (bind _asroots_of_shadows_game_state (Utilities|Casting|CastToRootsOfShadowsGameState (Game|GetGameInstance)))
  (Variables|Default|SetROS%20Game%20Instance _asroots_of_shadows_game_state))

(event Collision|EventActorBeginOverlap
  (params (OtherActor :type Actor%20Object%20Reference)))

(event EventTick
  (params (DeltaSeconds :type Float%20%28single-precision%29))
  ;[1 1 1] Set Selection Mode
  (Rendering|SetVisibility (Variables|Default|GetSelectionUI) (Variables|Default|GetbIsSelected) false)
  (CallFunction|QuestUIFacingPlayer))

(event EventOnQuestUIChanged
  (CallFunction|SetVisibleQuestUI))

(fn ConstructionScript)

(fn GEFacingPlayer
  (bind _gequestui (Variables|Default|GetGEQuestUI))
  (if (Variables|/Script/Engine.SceneComponent|GetbVisible _gequestui)
    (Transformation|SetWorldRotation _gequestui (Math|Rotator|FindLookatRotation (Transformation|GetWorldLocation (Variables|Default|GetGEQuestUI)) (Transformation|GetActorLocation (Game|GetPlayerCameraManager 0))) false false)))

(fn GIFacingPlayer
  (bind _giquestui (Variables|Default|GetGIQuestUI))
  (if (Variables|/Script/Engine.SceneComponent|GetbVisible _giquestui)
    (Transformation|SetWorldRotation _giquestui (Math|Rotator|FindLookatRotation (Transformation|GetWorldLocation (Variables|Default|GetGIQuestUI)) (Transformation|GetActorLocation (Game|GetPlayerCameraManager 0))) false false)))

(fn YEFacingPlayer
  (bind _yequestui (Variables|Default|GetYEQuestUI))
  (if (Variables|/Script/Engine.SceneComponent|GetbVisible _yequestui)
    (Transformation|SetWorldRotation _yequestui (Math|Rotator|FindLookatRotation (Transformation|GetWorldLocation (Variables|Default|GetYEQuestUI)) (Transformation|GetActorLocation (Game|GetPlayerCameraManager 0))) false false)))

(fn YIFacingPlayer
  (bind _yiquestui (Variables|Components|GetYIQuestUI))
  (if (Variables|/Script/Engine.SceneComponent|GetbVisible _yiquestui)
    (Transformation|SetWorldRotation _yiquestui (Math|Rotator|FindLookatRotation (Transformation|GetWorldLocation (Variables|Components|GetYIQuestUI)) (Transformation|GetActorLocation (Game|GetPlayerCameraManager 0))) false false)))

(fn QuestUIFacingPlayer
  (CallFunction|GEFacingPlayer)
  (CallFunction|GIFacingPlayer)
  (CallFunction|YEFacingPlayer)
  (CallFunction|YIFacingPlayer))

(fn SetVisibleQuestUI
  (Rendering|SetVisibility (Variables|Default|GetGEQuestUI) false false)
  (switch string (Variables|Default|GetQuestState)
    (:GE
      (Rendering|SetVisibility (Variables|Default|GetGEQuestUI) true false))
    (:GI
      (Rendering|SetVisibility (Variables|Default|GetGIQuestUI) true false))
    (:YE
      (Rendering|SetVisibility (Variables|Default|GetYEQuestUI) true false))
    (:YI
      (Rendering|SetVisibility (Variables|Components|GetYIQuestUI) true false))))