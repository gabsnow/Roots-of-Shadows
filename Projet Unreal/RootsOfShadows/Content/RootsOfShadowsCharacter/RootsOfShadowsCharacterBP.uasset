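; Player character Blueprint for Roots of Shadows that connects character events to the HUD, NPC dialog, quest updates and death menu.
; BeginPlay builds the HUD from game-instance data, delaying it for an unviewed cinematic and respawning at zero health.
; Health, mana and exp changes save position through the game instance, while a Tick-driven Delay paces regeneration.
; Attack animation chains and an unfinished quest lookup are unwired and never run.
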(event EventBeginPlay
  (|CallParentFunction)
  (Widget|SetVisibility (UserInterface|GetUserWidgetObject (Variables|Default|GetQuestUI)) "Collapsed")
  (Variables|Default|SetauthorizeMagic true)
  (Variables|Default|SetauthorizeAttack1 true)
  (Variables|Default|SetauthorizeAttack2 true)
  (bind _asroots_of_shadows_game_state (Utilities|Casting|CastToRootsOfShadowsGameState (Game|GetGameInstance)))
  (bind _output_get (Variables|Default|SetROSGameInstance _asroots_of_shadows_game_state))
  (Variables|Default|SetDatabasePlayer (Variables|/Script/RootsOfShadows.RootsOfShadowsGameState|GetDatabasePlayer _output_get))
  (bind _returnvalue (UserInterface|CreateWidget "/Game/UIs/MainGUI.MainGUI_C"))
  (bind _output_get_2 (Variables|Default|SetROSMainGUI _returnvalue))
  (Default|SetQuestUI _output_get_2)
  (if (.bCinematicViewed (Utilities|Struct|BreakDBPlayer (Variables|Default|GetDatabasePlayer)))
    _
    (else
      (Utilities|FlowControl|Delay 54.299999)))
  (CallFunction|AddMainGUI)
  (if (<= (.Health (Utilities|Struct|BreakDBPlayer (Variables|/Script/RootsOfShadows.RootsOfShadowsGameState|GetDatabasePlayer (Variables|Default|GetROSGameInstance)))) 0.0)
    (Class|RootsOfShadowsCharacter|Respawn)))

(event Collision|EventActorBeginOverlap
  (params (OtherActor :type Actor%20Object%20Reference))
  (|CallParentFunction OtherActor) ; This node is disabled and will not be called.\nDrag off pins to build functionality.
)

(event EventOnQuestProgress
  (Default|SetQuestUI (Variables|Default|GetROSMainGUI)))

(event EventOnSpecialAttackCast
  ;[1 1 1] Cooldowns
  (Default|SetSpecialCooldown (Variables|Default|GetROSMainGUI)))

(event EventOnSpecialAttackCooledDown
  ;[1 1 1] Cooldowns
  (Default|ResetSpecialCooldown (Variables|Default|GetROSMainGUI)))

(event EventOnMagicAttackCast
  ;[1 1 1] Cooldowns
  (Default|SetMagicCooldown (Variables|Default|GetROSMainGUI)))

(event EventOnMagicAttackCooledDown
  ;[1 1 1] Cooldowns
  (Default|ResetMagicCooldown (Variables|Default|GetROSMainGUI)))

(event EventTick
  (params (DeltaSeconds :type Float%20%28single-precision%29))
  ;[1 1 1] Health & Mana Regen
  (|CallParentFunction DeltaSeconds)
  (Variables|Default|SetPlayerActualPosition (Transformation|GetActorLocation (Game|Player|GetPlayerPawn 0)))
  (Default|SetQuestUI (Variables|Default|GetROSMainGUI))
  (Utilities|FlowControl|Delay 5.0)
  (Class|RootsOfShadowsCharacter|Regeneration))

(event EventOnSelectedNpcChanged
  ;[1 1 1] Montrer le quest UI
  (bind _asnpccharacter_bp (Utilities|Casting|CastToNPCCharacterBP (Variables|Default|GetTarget)))
  (if (not (== (Utilities|Array|Length (Variables|/Script/RootsOfShadows.NPCCharacter|GetDialogTexts _asnpccharacter_bp)) 0))
    (Widget|SetVisibility (UserInterface|GetUserWidgetObject (Variables|Default|GetQuestUI)) "Visible")
    (Variables|Default|SetbQuestUIIsOpen true)
    (bind _asdialog_gui (Utilities|Casting|CastToDialogGUI (UserInterface|GetUserWidgetObject (Variables|Default|GetQuestUI))))
    (Default|DialogUIInitText _asdialog_gui _asnpccharacter_bp)))

(event EventOnHealthChanged
  ;[1 1 1] Update PlayerInfo
  (Default|SetPlayerHealth (Variables|Default|GetROSMainGUI))
  (CallFunction|UpdatePlayerLocation))

(event EventOnManaChanged
  ;[1 1 1] Update PlayerInfo
  (Default|SetPlayerMana (Variables|Default|GetROSMainGUI))
  (CallFunction|UpdatePlayerLocation))

(event EventOnExpChanged
  ;[1 1 1] Update PlayerInfo
  (Default|SetPlayerExp (Variables|Default|GetROSMainGUI))
  (CallFunction|UpdatePlayerLocation))

(event EventOnDie
  ;[1 1 1] Player Death
  (Utilities|FlowControl|Delay 1.0)
  (bind _returnvalue (UserInterface|CreateWidget "/Game/UIs/DeathMenuGUI.DeathMenuGUI_C"))
  (UserInterface|Viewport|AddtoViewport _returnvalue 0))

(event EventWeGotTooFarfromNPC
  ;[1 1 1] Montrer le quest UI
  (Widget|SetVisibility (UserInterface|GetUserWidgetObject (Variables|Default|GetQuestUI)) "Collapsed")
  (Variables|Default|SetbQuestUIIsOpen false))

(event EventOnQuestComplete
  (CallFunction|SetQuestUIs)
  (Default|SetQuestUI (Variables|Default|GetROSMainGUI)))

(event Input|KeyboardEvents|Escape
  (params (Key :type Key%20Structure))
  (:Pressed
    (Default|ToggleMenu (Variables|Default|GetROSMainGUI))))

(event Input|KeyboardEvents|3
  (params (Key :type Key%20Structure))
  ;[1 1 1] MagicAttack Animation
)

(event Input|KeyboardEvents|2
  (params (Key :type Key%20Structure))
  ;[1 1 1] Attack2 Animation
)

(event Input|KeyboardEvents|1
  (params (Key :type Key%20Structure))
  ;[1 1 1] Attack1 Animation
)

(fn ConstructionScript
  (|CallParentFunction))

(fn AddMainGUI
  (UserInterface|Viewport|AddtoViewport (Variables|Default|GetROSMainGUI) 0))

(fn RemoveMainGUI
  (Widget|RemovefromParent (Variables|Default|GetROSMainGUI)))

(fn UpdatePlayerLocation
  (bind _rosgameinstance (Variables|Default|GetROSGameInstance))
  (bind _structout (Utilities|Struct|SetmembersinDBPlayer (Variables|/Script/RootsOfShadows.RootsOfShadowsGameState|GetDatabasePlayer _rosgameinstance) (Transformation|GetActorLocation)))
  (Variables|/Script/RootsOfShadows.RootsOfShadowsGameState|SetDatabasePlayer _rosgameinstance _structout)
  (Class|RootsOfShadowsGameState|UpdatePlayer _rosgameinstance))

(fn SetQuestUIs
  (bind _outactors (Actor|GetAllActorsOfClass "/Script/RootsOfShadows.NPCCharacter"))
  (for _array_element _outactors
    (Class|NPCCharacter|SetQuest _array_element)))