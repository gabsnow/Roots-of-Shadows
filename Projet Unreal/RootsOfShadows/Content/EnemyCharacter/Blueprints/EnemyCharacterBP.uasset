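; Enemy character Blueprint that shows a world-space health bar and a selection indicator.
; It refreshes the health bar widget from the HealthComponent's current and max health on BeginPlay and whenever health changes.
; Each Tick turns the health bar toward the player camera and shows or hides SelectionUI based on the IsSelected flag.
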(event EventBeginPlay
  (CallFunction|UpdateHealth))

(event Collision|EventActorBeginOverlap
  (params (OtherActor :type Actor%20Object%20Reference)))

(event EventTick
  (params (DeltaSeconds :type Float%20%28single-precision%29))
  ;[1 1 1] HealthBar Facing Player
  (Transformation|SetWorldRotation (Variables|Default|GetHealthBarComp) (Math|Rotator|FindLookatRotation (Transformation|GetWorldLocation (Variables|Default|GetHealthBarComp)) (Transformation|GetActorLocation (Game|GetPlayerCameraManager 0))) false false)
  ;[1 1 1] Set Selection Mode
  (Rendering|SetVisibility (Variables|Default|GetSelectionUI) (Variables|Default|GetbIsSelected) false))

(event EventOnHealthChanged
  (CallFunction|UpdateHealth))

(fn ConstructionScript)

(fn UpdateHealth
  (bind _healthcomponent (Variables|Default|GetHealthComponent))
  (bind _asenemy_health_bar_gui (Utilities|Casting|CastToEnemyHealthBarGUI (UserInterface|GetUserWidgetObject (Variables|Default|GetHealthBarComp))))
  (Default|SetHealthProgress _asenemy_health_bar_gui (Variables|/Script/RootsOfShadows.HealthComponent|GetHealth _healthcomponent) (Variables|/Script/RootsOfShadows.HealthComponent|GetMaxHealth _healthcomponent)))