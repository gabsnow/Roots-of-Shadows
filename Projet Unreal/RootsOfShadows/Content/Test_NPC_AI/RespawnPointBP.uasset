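; RespawnPointBP is a checkpoint trigger that saves a respawn location for the player.
; Any begin overlap on its Box stores player 0's current character location, without checking which actor entered.
; It writes that location into a RespawnCoordinate SaveGame in the "RespawnPoint" slot, updating the existing save or creating one if none exists.
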(event OnComponentBeginOverlap(Box)
  (params (OverlappedComponent :type Primitive%20Component%20Object%20Reference) (OtherActor :type Actor%20Object%20Reference) (OtherComp :type Primitive%20Component%20Object%20Reference) (OtherBodyIndex :type Integer) (bFromSweep :type Boolean) (SweepResult :type Hit%20Result%20Structure%20%28by%20ref%29))
  (Utilities|FlowControl|Sequence
    (:then_0
      (bind _asroots_of_shadows_character (Utilities|Casting|CastToRootsOfShadowsCharacter (Game|GetPlayerCharacter 0)))
      (Variables|Default|SetRespawnCoordinate (Transformation|GetActorLocation _asroots_of_shadows_character)))
    (:then_1
      (bind _returnvalue (SaveGame|DoesSaveGameExist "RespawnPoint"))
      (if _returnvalue
        (bind _returnvalue_2 (SaveGame|LoadGamefromSlot "RespawnPoint"))
        (bind _asrespawn_coordinate (Utilities|Casting|CastToRespawnCoordinate _returnvalue_2))
        (Variables|/Game/Test_NPC_AI/RespawnCoordinate.RespawnCoordinate_C|SetSpawnCoordinate _asrespawn_coordinate (Variables|Default|GetRespawnCoordinate))
        (SaveGame|SaveGametoSlot _asrespawn_coordinate "RespawnPoint")
        (else
          (bind _returnvalue_3 (SaveGame|CreateSaveGameObject "/Game/Test_NPC_AI/RespawnCoordinate.RespawnCoordinate_C"))
          (Variables|/Game/Test_NPC_AI/RespawnCoordinate.RespawnCoordinate_C|SetSpawnCoordinate _returnvalue_3 (Variables|Default|GetRespawnCoordinate))
          (SaveGame|SaveGametoSlot _returnvalue_3 "RespawnPoint"))))))

(event EventBeginPlay)

(event Collision|EventActorBeginOverlap
  (params (OtherActor :type Actor%20Object%20Reference)))

(event EventTick
  (params (DeltaSeconds :type Float%20%28single-precision%29)))

(fn ConstructionScript)